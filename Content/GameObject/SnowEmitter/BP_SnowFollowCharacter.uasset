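; Snow emitter actor that keeps its particle system above the player so the effect follows them through the world.
; On BeginPlay it caches player pawn 0 and enables following if that pawn is valid.
; Each Tick then moves only the particle system component to the pawn's world location with a fixed upward offset, without rechecking validity.
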(event EventTick
  (params (DeltaSeconds :type Float%20%28single-precision%29))
  (bind _actortofollow (Variables|Default|GetActorToFollow))
  (bind _returnvalue (Transformation|GetActorLocation _actortofollow))
  (if (Variables|Default|GetIsFollowingActor)
    (Transformation|SetWorldLocation (Variables|Default|GetParticleSystem) (Math|Vector|MakeVector (.x _returnvalue) (.y _returnvalue) (+ (.z _returnvalue) 4e+02)) false false)))

(event EventBeginPlay
  (Variables|Default|SetActorToFollow (Game|Player|GetPlayerPawn 0))
  (Utilities|IsValid (Variables|Default|GetActorToFollow)
    (:Is%20Valid
      (Variables|Default|SetIsFollowingActor true))))

(fn ConstructionScript)