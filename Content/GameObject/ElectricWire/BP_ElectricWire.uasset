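; BP_ElectricWire is an electric wire actor whose cable shows whether it is powered.
; Each ActivateAction event alternates the Powered flag through a FlipFlop, starting with on.
; Tick polls that flag and swaps the cable's first material between PoweredOn and PoweredOff, only when the current material does not already match.
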(event EventBeginPlay)

(event Collision|EventActorBeginOverlap
  (params (OtherActor :type Actor%20Object%20Reference)))

(event EventTick
  (params (DeltaSeconds :type Float%20%28single-precision%29))
  (bind _poweredon (Variables|Default|GetPoweredOn))
  (if (and (Variables|Default|GetPowered) (!= (Rendering|Material|GetMaterial (Variables|Default|GetCable) 0) _poweredon))
    (Rendering|Material|SetMaterial (Variables|Default|GetCable) 0 _poweredon)
    (elif (and (not (Variables|Default|GetPowered)) (!= (Rendering|Material|GetMaterial (Variables|Default|GetCable) 0) (Variables|Default|GetPoweredOff)))
      (Rendering|Material|SetMaterial (Variables|Default|GetCable) 0 (Variables|Default|GetPoweredOff)))))

(event EventActivateAction
  (Utilities|FlowControl|FlipFlop
    (:A
      (Variables|Default|SetPowered true))
    (:B
      (Variables|Default|SetPowered false))))

(fn ConstructionScript)