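; BP_UnlockLaser is an unlock object that grants the player the laser.
; On ActivateAction it casts player pawn 0 to ThirdPersonCharacter, calls UnlockLaser on it, then runs FollowUpAction.
; If the cast fails, neither call happens.
; BeginPlay, overlap and tick are disabled stubs, and the construction script only calls its parent.
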(event EventBeginPlay
  (|CallParentFunction) ; This node is disabled and will not be called.\nDrag off pins to build functionality.
)

(event Collision|EventActorBeginOverlap
  (params (OtherActor :type Actor%20Object%20Reference))
  (|CallParentFunction OtherActor) ; This node is disabled and will not be called.\nDrag off pins to build functionality.
)

(event EventTick
  (params (DeltaSeconds :type Float%20%28single-precision%29))
  (|CallParentFunction DeltaSeconds) ; This node is disabled and will not be called.\nDrag off pins to build functionality.
)

(event EventActivateAction
  (bind _asthird_person_character (Utilities|Casting|CastToThirdPersonCharacter (Game|Player|GetPlayerPawn 0)))
  (Default|UnlockLaser _asthird_person_character)
  (CallFunction|FollowUpAction))

(fn ConstructionScript
  (|CallParentFunction))