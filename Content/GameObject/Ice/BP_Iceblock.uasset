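; BP_Iceblock is an ice block actor that melts by shrinking its vertical scale in steps.
; Each ActivateAction calls MeltTo with TargetSize lowered by a fixed amount, which restarts the melt Alpha.
; Tick advances Alpha by MeltSpeed and lerps Z from the current scale toward the initial scale times TargetSize, giving a non-linear ease while X and Y stay fixed.
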(event Custom|MeltTo
  (params (Amount :type Float%20%28single-precision%29))
  (Variables|Default|SetTargetSize Amount)
  (Variables|Default|SetAlpha 0.0))

(event EventBeginPlay
  (Variables|Default|SetInitialScale (Transformation|GetWorldScale (Variables|Default|GetDefaultSceneRoot))))

(event EventTick
  (params (DeltaSeconds :type Float%20%28single-precision%29))
  (bind _initialscale (Variables|Default|GetInitialScale))
  (if (<= (Variables|Default|GetAlpha) 1.0)
    (Variables|Default|SetAlpha (+ (Variables|Default|GetAlpha) (* DeltaSeconds (Variables|Default|GetMeltSpeed))))
    (Transformation|SetActorScale3D (Math|Vector|MakeVector (.x _initialscale) (.y _initialscale) (.Z (Math|Vector|BreakVector (Math|Vector|Lerp(Vector) (Transformation|GetActorScale3D) (* (Variables|Default|GetInitialScale) (Variables|Default|GetTargetSize)) (Variables|Default|GetAlpha))))))))

(event EventActivateAction
  (CallFunction|Meltto (- (Variables|Default|GetTargetSize) 0.5)))

(fn ConstructionScript)