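; BP_IceBlockManager is a manager that triggers all ice blocks in the level at once and adjusts the snow on an ice melt tower.
; On BeginPlay it caches every BP_Iceblock actor in an array.
; ActivateAction forwards the call to each cached block, then doubles the referenced IceMeltTower's snow distance threshold and lowers its snow amount by a fixed step.
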(event EventBeginPlay
  (bind _outactors (Actor|GetAllActorsOfClass "/Game/GameObject/Ice/BP_Iceblock.BP_Iceblock_C"))
  (Variables|Default|SetIceBlocks _outactors))

(event Collision|EventActorBeginOverlap
  (params (OtherActor :type Actor%20Object%20Reference)))

(event EventTick
  (params (DeltaSeconds :type Float%20%28single-precision%29)))

(event EventActivateAction
  (bind _icemelttower (Variables|Default|GetIceMeltTower))
  (for _array_element (Variables|Default|GetIceBlocks)
    (Default|ActivateAction _array_element))
  (Variables|/Game/ThirdPersonBP/Blueprints/TowerLocation_Blueprint.TowerLocation_Blueprint_C|SetSnowDistanceThreshold _icemelttower (* (Variables|/Game/ThirdPersonBP/Blueprints/TowerLocation_Blueprint.TowerLocation_Blueprint_C|GetSnowDistanceThreshold _icemelttower) 2.0))
  (Variables|/Game/ThirdPersonBP/Blueprints/TowerLocation_Blueprint.TowerLocation_Blueprint_C|SetSnowAmount _icemelttower (- (Variables|/Game/ThirdPersonBP/Blueprints/TowerLocation_Blueprint.TowerLocation_Blueprint_C|GetSnowAmount _icemelttower) 0.5)))

(fn ConstructionScript)