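; Tower actor that holds four power cores (Start, Magnet, Laser and Last) and can push out a chosen one.
; PushOutCore maps the core type to its component through GetCoreReference, then uses MoveComponentTo to slide it up and along local Y over a few seconds, keeping its rotation.
; The target is an offset from the core's current relative location.
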(event Custom|PushOutCore
  (params (WhichCore :type Cores%20Enum :default "NewEnumerator0"))
  (bind _reference (CallFunction|GetCoreReference WhichCore))
  (Components|MoveComponentTo _reference (Math|Vector|MakeVector (.x (.location (Transformation|GetRelativeTransform _reference))) (+ (.y (.location (Transformation|GetRelativeTransform _reference))) 5e+01) (+ (.z (.location (Transformation|GetRelativeTransform _reference))) 1.1e+02)) (.rotation (Transformation|GetRelativeTransform _reference)) false false 5.0 false))

(event EventBeginPlay)

(event Collision|EventActorBeginOverlap
  (params (OtherActor :type Actor%20Object%20Reference)))

(event EventTick
  (params (DeltaSeconds :type Float%20%28single-precision%29)))

(fn ConstructionScript)

(fn GetCoreReference
  (params (WhichCore :type Cores%20Enum :default "NewEnumerator0"))
  (switch Utilities|FlowControl|Switch|SwitchonCores WhichCore
    (:NewEnumerator0
      (return (Variables|Default|GetPowerCore1)))
    (:NewEnumerator1
      (return (Variables|Default|GetPowerCore2)))
    (:NewEnumerator2
      (return (Variables|Default|GetPowerCore3)))
    (:NewEnumerator3
      (return (Variables|Default|GetPowerCore4)))))