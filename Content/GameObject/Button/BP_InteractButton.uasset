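; One-shot interactable button or lever that sends ActivateActionMessage to a referenced actor.
; The construction script selects button or lever visuals, key-press or pressure trigger mode, and can aim a debug arrow at the target.
; Key mode shows a billboard nearby and binds the character's Interact event; pressure mode fires on overlap by the character or an optional designated actor.
; Activation animates the mesh, and a separate trigger box drives custom-depth highlighting.
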(event OnComponentBeginOverlap(PressureTriggerBox)
  (params (OverlappedComponent :type Primitive%20Component%20Object%20Reference) (OtherActor :type Actor%20Object%20Reference) (OtherComp :type Primitive%20Component%20Object%20Reference) (OtherBodyIndex :type Integer) (bFromSweep :type Boolean) (SweepResult :type Hit%20Result%20Structure%20%28by%20ref%29))
  (bind _buttonmesh (Variables|Default|GetButtonMesh))
  (bind _leverbars (Variables|Default|GetLeverBars))
  (bind _returnvalue (Transformation|GetRelativeTransform _buttonmesh))
  (bind _returnvalue_2 (Transformation|GetRelativeTransform _leverbars))
  (bind (_x _y _z) (Math|Vector|BreakVector (.location _returnvalue)))
  (bind (_roll _pitch _yaw) (Math|Rotator|BreakRotator (.rotation _returnvalue_2)))
  (if (and (== OtherActor (Variables|ActorInteractAble|GetPressableActor)) (Variables|ActorInteractAble|GetCanOtherActorInteract))
    _
    (else
      (Utilities|Casting|CastToThirdPersonCharacter OtherActor)))
  (if (and (Variables|Default|GetIsInteractable) (Utilities|CanInteractwithCharacter))
    ;[1 1 1] MoveButtonMesh down with timer
    (Variables|Default|SetIsInteractable false)
    (if (Variables|Default|GetIsLever)
      (Components|MoveComponentTo _leverbars (.location _returnvalue_2) (Math|Rotator|MakeRotator (+ _roll 9e+01) _pitch _yaw) false false 1.0 false)
      (else
        (Components|MoveComponentTo _buttonmesh (Math|Vector|MakeVector _x _y (+ _z -1e+01)) (.rotation _returnvalue) false false 1.0 false)))
    (Rendering|Material|SetMaterial (Variables|Default|GetButtonMesh) 0 "/Game/GameObject/Button/ButtonMaterial/M_PressedMaterial.M_PressedMaterial")
    (Class|BPIActivatable|ActivateAction(Message) (Variables|Linking|GetActorReference))))

(event OnComponentBeginOverlap(HighLightTriggerBox)
  (params (OverlappedComponent :type Primitive%20Component%20Object%20Reference) (OtherActor :type Actor%20Object%20Reference) (OtherComp :type Primitive%20Component%20Object%20Reference) (OtherBodyIndex :type Integer) (bFromSweep :type Boolean) (SweepResult :type Hit%20Result%20Structure%20%28by%20ref%29))
  (Utilities|Casting|CastToThirdPersonCharacter OtherActor)
  (Rendering|SetRenderCustomDepth (Variables|Default|GetBaseMesh) true))

(event OnComponentBeginOverlap(KeyPressTriggerBox)
  (params (OverlappedComponent :type Primitive%20Component%20Object%20Reference) (OtherActor :type Actor%20Object%20Reference) (OtherComp :type Primitive%20Component%20Object%20Reference) (OtherBodyIndex :type Integer) (bFromSweep :type Boolean) (SweepResult :type Hit%20Result%20Structure%20%28by%20ref%29))
  (Utilities|Casting|CastToThirdPersonCharacter OtherActor)
  (if (Utilities|CanInteractwithCharacter)
    (Variables|KeyInteraction|SetIsCharacterClose true)
    (Rendering|SetVisibility (Variables|Default|GetMaterialBillboard) true false)))

(event OnComponentEndOverlap(KeyPressTriggerBox)
  (params (OverlappedComponent :type Primitive%20Component%20Object%20Reference) (OtherActor :type Actor%20Object%20Reference) (OtherComp :type Primitive%20Component%20Object%20Reference) (OtherBodyIndex :type Integer))
  (Utilities|Casting|CastToThirdPersonCharacter OtherActor)
  (Variables|KeyInteraction|SetIsCharacterClose false)
  (Rendering|SetVisibility (Variables|Default|GetMaterialBillboard) false false))

(event OnComponentEndOverlap(HighLightTriggerBox)
  (params (OverlappedComponent :type Primitive%20Component%20Object%20Reference) (OtherActor :type Actor%20Object%20Reference) (OtherComp :type Primitive%20Component%20Object%20Reference) (OtherBodyIndex :type Integer))
  (Utilities|Casting|CastToThirdPersonCharacter OtherActor)
  (Rendering|SetRenderCustomDepth (Variables|Default|GetBaseMesh) false))

(event Custom|ButtonInteract
  (bind _leverbars (Variables|Default|GetLeverBars))
  (bind _buttonmesh (Variables|Default|GetButtonMesh))
  (bind _returnvalue (Transformation|GetRelativeTransform _buttonmesh))
  (bind _returnvalue_2 (Transformation|GetRelativeTransform _leverbars))
  (bind (_x _y _z) (Math|Vector|BreakVector (.location _returnvalue)))
  (bind (_roll _pitch _yaw) (Math|Rotator|BreakRotator (.rotation _returnvalue_2)))
  ;[1 1 1] InputAction Interact: If Interactable and Character close, press button and activatable
  (if (and (Variables|Default|GetIsInteractable) (Variables|KeyInteraction|GetIsCharacterClose))
    (Variables|Default|SetIsInteractable false)
    (Rendering|SetVisibility (Variables|Default|GetMaterialBillboard) false false)
    (if (Variables|Default|GetIsLever)
      (Components|MoveComponentTo _leverbars (.location _returnvalue_2) (Math|Rotator|MakeRotator (+ _roll 9e+01) _pitch _yaw) false false 1.0 false)
      (else
        (Components|MoveComponentTo _buttonmesh (Math|Vector|MakeVector _x _y (+ _z -1e+01)) (.rotation _returnvalue) false false 1.0 false)))
    (Rendering|Material|SetMaterial (Variables|Default|GetButtonMesh) 0 "/Game/GameObject/Button/ButtonMaterial/M_PressedMaterial.M_PressedMaterial")
    (Class|BPIActivatable|ActivateAction(Message) (Variables|Linking|GetActorReference))))

(event EventBeginPlay
  ;[1 1 1] BeginPlay: Check if reference valid and print debug line if true
  (Utilities|IsValid (Variables|Linking|GetActorReference)
    (:Is%20Valid
      (bind _asthird_person_character (Utilities|Casting|CastToThirdPersonCharacter (Game|Player|GetPlayerPawn 0)))
      (EventDispatchers|BindEventtoInteract _asthird_person_character (delegate Custom|ButtonInteract)))
    (:Is%20Not%20Valid
      (Development|PrintString (Utilities|String|Append (Utilities|GetDisplayName self) "'s ActorReference is not set!!!") true false "(R=1.000000,G=0.018540,B=0.000000,A=1.000000)" 1e+01))))

(fn ConstructionScript
  (bind _islever (Variables|Default|GetIsLever))
  (bind _actorreference (Variables|Linking|GetActorReference))
  (bind _arrow (Variables|Default|GetArrow))
  (bind _pressurebutton (Variables|Default|GetPressureButton))
  (bind _returnvalue (Transformation|GetActorLocation _actorreference))
  (bind _returnvalue_2 (Transformation|GetWorldLocation _pressurebutton))
  (CallFunction|SetOverlapBoxes)
  (Rendering|SetVisibility (Variables|Default|GetLeverBase) _islever true)
  (Rendering|SetVisibility (Variables|Default|GetBaseMesh) (not _islever) true)
  (if (Variables|Linking|GetDrawDebugLine)
    (Transformation|SetWorldScale3D _arrow (Math|Vector|MakeVector (* (Math|Vector|VectorLength (- _returnvalue_2 _returnvalue)) 0.01) 1.0 1.0))
    (Transformation|SetWorldLocationAndRotation _arrow _returnvalue_2 (Math|Rotator|FindLookatRotation _returnvalue_2 _returnvalue) false true)))

(fn SetOverlapBoxes
  (bind _keypresstriggerbox (Variables|Default|GetKeyPressTriggerBox))
  (bind _pressuretriggerbox (Variables|Default|GetPressureTriggerBox))
  (bind _keypresstriggerbox_2 (Variables|Default|GetKeyPressTriggerBox))
  (bind _pressuretriggerbox_2 (Variables|Default|GetPressureTriggerBox))
  (if (Variables|Interaction|GetIsKeyPressButton)
    (Variables|/Script/Engine.PrimitiveComponent|SetbGenerateOverlapEvents _keypresstriggerbox_2 true)
    (Rendering|SetVisibility _keypresstriggerbox_2 true false)
    (Variables|/Script/Engine.PrimitiveComponent|SetbGenerateOverlapEvents _pressuretriggerbox_2 false)
    (Rendering|SetVisibility _pressuretriggerbox_2 false false)
    (Variables|ActorInteractAble|SetCanOtherActorInteract false)
    (Variables|ActorInteractAble|SetPressableActor 0)
    (else
      (Variables|/Script/Engine.PrimitiveComponent|SetbGenerateOverlapEvents _keypresstriggerbox false)
      (Rendering|SetVisibility _keypresstriggerbox false false)
      (Variables|/Script/Engine.PrimitiveComponent|SetbGenerateOverlapEvents _pressuretriggerbox true)
      (Rendering|SetVisibility _pressuretriggerbox true false))))

(fn MoveButtonDown)