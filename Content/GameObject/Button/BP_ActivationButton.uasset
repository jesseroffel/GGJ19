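; BP_ActivationButton is a button that activates a referenced actor when anything overlaps its TriggerBox.
; Activate sets the target's IsActivated flag and calls its ActivationFunction, skipping targets that are already activated.
; On BeginPlay it can draw a debug line from the button to the target's LocationPoint, or prints an on-screen warning if ActorReference is invalid.
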(event OnComponentBeginOverlap(TriggerBox)
  (params (OverlappedComponent :type Primitive%20Component%20Object%20Reference) (OtherActor :type Actor%20Object%20Reference) (OtherComp :type Primitive%20Component%20Object%20Reference) (OtherBodyIndex :type Integer) (bFromSweep :type Boolean) (SweepResult :type Hit%20Result%20Structure%20%28by%20ref%29))
  (Utilities|IsValid (Variables|Linking|GetActorReference)
    (:Is%20Valid
      (CallFunction|Activate))))

(event EventBeginPlay
  ;[1 1 1] BeginPlay: Check if reference valid and print debug line if true
  (Utilities|IsValid (Variables|Linking|GetActorReference)
    (:Is%20Valid
      (if (Variables|Linking|GetDrawDebugLine)
        (Rendering|Debug|DrawDebugLine (Transformation|GetWorldLocation (Variables|Default|GetButton)) (Transformation|GetWorldLocation (Variables|/Game/GameObject/Button/BP_ActivatableTemplate.BP_ActivatableTemplate_C|GetLocationPoint (Variables|Linking|GetActorReference))) "(R=0.687500,G=0.638433,B=0.043884,A=1.000000)" 5e+01 3.0)))
    (:Is%20Not%20Valid
      (Development|PrintString (Utilities|String|Append (Utilities|GetDisplayName self) "'s ActorReference is not set!!!") true false "(R=1.000000,G=0.018540,B=0.000000,A=1.000000)" 1e+01))))

(fn ConstructionScript)

(fn Activate
  (bind _actorreference (Variables|Linking|GetActorReference))
  (if (not (Variables|/Game/GameObject/Button/BP_ActivatableTemplate.BP_ActivatableTemplate_C|GetIsActivated _actorreference))
    (Variables|/Game/GameObject/Button/BP_ActivatableTemplate.BP_ActivatableTemplate_C|SetIsActivated _actorreference true)
    (Default|ActivationFunction (Variables|Linking|GetActorReference))))