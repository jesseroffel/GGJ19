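; BP_LaserButton is a laser receiver button that activates a linked TargetActor when hit.
; Its Hit event slides the cylinder inward, swaps it to the active receiver material and turns the point light green.
; It then sends ActivateActionMessage to TargetActor through an interface check, keeping the target type generic.
; With DrawDebugLine enabled, the construction script stretches and aims an arrow at TargetActor to visualize the link.
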(event Custom|Hit
  (bind _cylinder (Variables|Default|GetCylinder))
  (bind _targetactor (Variables|Default|GetTargetActor))
  (Components|MoveComponentTo _cylinder "-20.000000, 0, 0" (Variables|/Script/Engine.SceneComponent|GetRelativeRotation _cylinder) false false 1.0 false)
  (Rendering|Material|SetMaterial (Variables|Default|GetCylinder) 0 "/Game/GameObject/Laser/MM_LaserReceiverActive.MM_LaserReceiverActive")
  (Rendering|Components|Light|SetLightColor (Variables|Default|GetPointLight) "(R=0.000000,G=1.000000,B=0.014110,A=1.000000)" true)
  (if (Utilities|DoesObjectImplementInterface _targetactor 0)
    (Class|BPIActivatable|ActivateAction(Message) _targetactor)))

(fn ConstructionScript
  (bind _arrow (Variables|Default|GetArrow))
  (bind _targetactor (Variables|Default|GetTargetActor))
  (bind _defaultsceneroot (Variables|Default|GetDefaultSceneRoot))
  (bind _returnvalue (Transformation|GetActorLocation _targetactor))
  (bind _returnvalue_2 (Transformation|GetWorldLocation _defaultsceneroot))
  (if (Variables|Default|GetDrawDebugLine)
    (Transformation|SetWorldScale3D _arrow (Math|Vector|MakeVector (* (Math|Vector|VectorLength (- _returnvalue_2 _returnvalue)) 0.01) 1.0 1.0))
    (Transformation|SetWorldLocationAndRotation _arrow _returnvalue_2 (Math|Rotator|FindLookatRotation _returnvalue_2 _returnvalue) false true)))