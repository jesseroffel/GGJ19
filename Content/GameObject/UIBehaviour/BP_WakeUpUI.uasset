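; BP_WakeUpUI is an actor that shows the wake-up screen overlay when play begins.
; On BeginPlay it creates a UI_WakeUp widget for the first player controller, adds it to the viewport and starts its fade-out.
; It then immediately calls FollowUpAction, which is defined outside this graph.
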(event Collision|EventActorBeginOverlap
  (params (OtherActor :type Actor%20Object%20Reference))
  (|CallParentFunction OtherActor) ; This node is disabled and will not be called.\nDrag off pins to build functionality.
)

(event EventTick
  (params (DeltaSeconds :type Float%20%28single-precision%29))
  (|CallParentFunction DeltaSeconds) ; This node is disabled and will not be called.\nDrag off pins to build functionality.
)

(event EventBeginPlay
  (bind _returnvalue (UserInterface|CreateWidget "/Game/UI/UI_WakeUp.UI_WakeUp_C" (Game|GetPlayerController 0)))
  (UserInterface|Viewport|AddtoViewport _returnvalue 0)
  (Default|SetFadeOut _returnvalue)
  (CallFunction|FollowUpAction))

(fn ConstructionScript
  (|CallParentFunction))