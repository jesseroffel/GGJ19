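; Camera path actor that, when activated, plays a flythrough by moving the third-person character's own follow camera along a spline.
; ActivateAction saves the camera's world transform, raises a flag and calls FollowUpAction; Tick consumes the flag to start CameraFollow once.
; A timeline maps its value to spline distance, driving camera location and rotation while the character's IsInputEnabled is false, then restores both on finish.
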(event EventActivateAction
  (bind _asthird_person_character (Utilities|Casting|CastToThirdPersonCharacter (Game|Player|GetPlayerPawn 0)))
  (bind _output_get (Variables|Following|SetCharacterRef _asthird_person_character))
  (Variables|Following|SetCallFollowEvent true)
  (Variables|Following|SetPreviousCam (Transformation|GetWorldTransform (Variables|/Game/ThirdPersonBP/Blueprints/ThirdPersonCharacter.ThirdPersonCharacter_C|GetFollowCamera _output_get)))
  (CallFunction|FollowUpAction))

(event EventTick
  (params (DeltaSeconds :type Float%20%28single-precision%29))
  (if (Variables|Following|GetCallFollowEvent)
    (Variables|Following|SetCallFollowEvent false)
    (CallFunction|CameraFollow)))

(event EventCameraFollow
  (bind _spline (Variables|Default|GetSpline))
  (Variables|/Game/ThirdPersonBP/Blueprints/ThirdPersonCharacter.ThirdPersonCharacter_C|SetIsInputEnabled (Variables|Following|GetCharacterRef) false)
  (Variables|Following|SetIsFollowingPath false)
  ;[1 1 1] I know.. timeline
  (bind _animation (Timeline|CameraFollowing PlayFromStart)
    (:Update
      (Transformation|SetWorldTransform (Variables|/Game/ThirdPersonBP/Blueprints/ThirdPersonCharacter.ThirdPersonCharacter_C|GetFollowCamera (Variables|Following|GetCharacterRef)) (Math|Transform|MakeTransform (Spline|GetLocationatDistanceAlongSpline _spline (* (Spline|GetSplineLength _spline) _animation) "World") (Spline|GetRotationatDistanceAlongSpline _spline (* (Spline|GetSplineLength _spline) _animation) "World")) false false))
    (:Finished
      (Transformation|SetWorldTransform (Variables|/Game/ThirdPersonBP/Blueprints/ThirdPersonCharacter.ThirdPersonCharacter_C|GetFollowCamera (Variables|Following|GetCharacterRef)) (Variables|Following|GetPreviousCam) false false)
      (Variables|/Game/ThirdPersonBP/Blueprints/ThirdPersonCharacter.ThirdPersonCharacter_C|SetIsInputEnabled (Variables|Following|GetCharacterRef) true))))

(fn ConstructionScript
  (|CallParentFunction))